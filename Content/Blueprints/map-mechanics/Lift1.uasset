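; Lift actor that moves to a target offset (LiftZielkoordinaten) from its starting position when something overlaps its trigger sphere.
; BeginPlay caches both endpoints, and a timeline lerps the whole actor between them without sweep.
; The sphere's begin overlap plays the timeline, while the actor-wide end overlap reverses it; both toggle the visibility of Licht1.
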(event `self.ReceiveBeginPlay`
  (bind _returnvalue (`self.K2_GetActorLocation` self))
  (set `self.World Loc` _returnvalue)
  (set `self.End Loc` (+ _returnvalue (`self.Lift-Zielkoordinaten`))))

(event `self.SphereCollision.OnComponentBeginOverlap`
  (params (OverlappedComponent :type "PrimitiveComponent Object Reference") (OtherActor :type "Actor Object Reference") (OtherComp :type "PrimitiveComponent Object Reference") (OtherBodyIndex :type Integer) (bFromSweep :type Boolean) (SweepResult :type "HitResult Structure (by ref)"))
  (`SceneComponent.ToggleVisibility` (`self.licht1`) false)
  (bind (_direction _lifttimeline) (`Timeline|Timeline_0` :!label _label)
    (:`Update`
      (`self.K2_SetActorRelativeLocation` (`KismetMathLibrary.VLerp` (`self.World Loc`) (`self.End Loc`) _lifttimeline)))))

(event `self.ReceiveActorEndOverlap`
  (params (OtherActor :type "Actor Object Reference"))
  (`SceneComponent.ToggleVisibility` (`self.licht1`) false)
  (goto _label :!via `Reverse`))

(fn `UserConstructionScript`)